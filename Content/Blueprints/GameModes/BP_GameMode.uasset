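; BP_GameMode is a game mode Blueprint that shows start and end screens for the game.
; StartGame creates WBP_StartGameWidget and adds it to the viewport.
; EndGame creates WBP_EndGameWidget and uses its WonGame flag to set a win or game-over message in green or red.
; BeginPlay, Tick and the construction script are empty, so both events depend on external callers.
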(event `self.StartGame`
  (bind _returnvalue (`|CreateWidget` "/Game/Blueprints/Widgets/WBP_StartGameWidget.WBP_StartGameWidget_C"))
  (`UserWidget.AddToViewport` _returnvalue 0))

(event `self.EndGame`
  (params (bWonGame :type Boolean))
  (bind _returnvalue (`|CreateWidget` "/Game/Blueprints/Widgets/WBP_EndGameWidget.WBP_EndGameWidget_C"))
  (`UserWidget.AddToViewport` _returnvalue 0)
  (`TextBlock.SetText` (`/Game/Blueprints/Widgets/WBP_EndGameWidget.StartGameText` _returnvalue) (select `bool` bWonGame :`false` "Game Over!!" :`true` "You Won!!" :!type "Text"))
  (set `/Game/Blueprints/Widgets/WBP_EndGameWidget.TextColor` (make `SlateColor` (select `bool` bWonGame :`false` (struct :`R` 0.941667 :`G` 0.121632 :`B` 0.129481 :`A` 1.0) :`true` (struct :`R` 0.142478 :`G` 0.95 :`B` 0.162256 :`A` 1.0) :!type "LinearColor Structure")) _returnvalue))

(fn `UserConstructionScript`)